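; Checkpoint actor that saves the player's position when its Trigger component is overlapped.
; On overlap it casts player character 0 to BP_Character_Ogre, stores its location and prints a debug message, without checking which actor overlapped.
; It then writes that location to a Save_Position object in the SaveSlot slot, loading the existing save or creating a new one if none exists.
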(event `self.Trigger.OnComponentBeginOverlap`
  (params (OverlappedComponent :type "PrimitiveComponent Object Reference") (OtherActor :type "Actor Object Reference") (OtherComp :type "PrimitiveComponent Object Reference") (OtherBodyIndex :type Integer) (bFromSweep :type Boolean) (SweepResult :type "HitResult Structure (by ref)"))
  (`|ExecutionSequence`
    (:`then_0`
      (bind _asbp_character_ogre (cast `/Game/Blueprint/Characters/BP_Character_Ogre` (`GameplayStatics.GetPlayerCharacter` 0)))
      (set `self.PLayerLocation` (`self.K2_GetActorLocation` _asbp_character_ogre))
      (`KismetSystemLibrary.PrintString` "CheckpointReached"))
    (:`then_1`
      (bind _returnvalue (`GameplayStatics.DoesSaveGameExist` (`self.SaveSlot`)))
      (if _returnvalue
        (bind _returnvalue_2 (`GameplayStatics.LoadGameFromSlot` (`self.SaveSlot`)))
        (bind _assave_position (cast `/Game/Blueprint/Checkpoint/Save_Position` _returnvalue_2))
        (set `/Game/Blueprint/Checkpoint/Save_Position.PlayerLocation` (`self.PLayerLocation`) _assave_position)
        (`GameplayStatics.SaveGameToSlot` _assave_position (`self.SaveSlot`))
        (else
          (bind _returnvalue_3 (`GameplayStatics.CreateSaveGameObject` "/Game/Blueprint/Checkpoint/Save_Position.Save_Position_C"))
          (set `/Game/Blueprint/Checkpoint/Save_Position.PlayerLocation` (`self.PLayerLocation`) _returnvalue_3)
          (`GameplayStatics.SaveGameToSlot` _returnvalue_3 (`self.SaveSlot`)))))))

(fn `UserConstructionScript`)