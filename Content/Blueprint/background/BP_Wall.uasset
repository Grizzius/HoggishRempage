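; BP_Wall is a modular 16m wall piece whose construction script picks its mesh from a WallType enum covering straight, corner, door, three-way, small and half variants.
; Per-type selects also set the mesh's relative offset for straight, door, half and small pieces, leaving corners and three-ways unmoved.
; A Windows flag swaps straight walls to a window mesh; its OnRep function is empty, and the event graph has no active logic.
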(fn `OnRep_Windows`)

(fn `UserConstructionScript`
  (`StaticMeshComponent.SetStaticMesh` (`self.WallMesh`) (select `/Game/Blueprint/background/Enum_Wall_Type` (`self.WallType`) :`NewEnumerator0` "/Game/StaticMesh/Wall_16m_straight.Wall_16m_straight" :`NewEnumerator1` "/Game/StaticMesh/Corner_16m.Corner_16m" :`NewEnumerator3` "/Game/StaticMesh/Wall_16m_doorsmall.Wall_16m_doorsmall" :`NewEnumerator4` "/Game/StaticMesh/Wall_DoorMedium_16m.Wall_DoorMedium_16m" :`NewEnumerator5` "/Game/StaticMesh/Wall_16m_BigDoor.Wall_16m_BigDoor" :`NewEnumerator6` "/Game/StaticMesh/3way1_16m.3way1_16m" :`NewEnumerator7` "/Game/StaticMesh/3Way2_16m.3Way2_16m" :`NewEnumerator8` "/Game/StaticMesh/wall_16m_small.wall_16m_small" :`NewEnumerator9` "/Game/StaticMesh/Wall_16m_half.Wall_16m_half" :!type "StaticMesh Object Reference"))
  (if (select `/Game/Blueprint/background/Enum_Wall_Type` (`self.WallType`) :`NewEnumerator0` true :`NewEnumerator3` true :`NewEnumerator4` true :`NewEnumerator5` true :`NewEnumerator9` true)
    (`SceneComponent.K2_SetRelativeLocation` (`self.WallMesh`) (0.0 5.0 400.0) false false)
    (if (and (`self.Windows`) (select `/Game/Blueprint/background/Enum_Wall_Type` (`self.WallType`) :`NewEnumerator0` true))
      (`StaticMeshComponent.SetStaticMesh` (`self.WallMesh`) "/Game/StaticMesh/Wall_16m_window.Wall_16m_window"))
    (elif (select `/Game/Blueprint/background/Enum_Wall_Type` (`self.WallType`) :`NewEnumerator8` true)
      (`SceneComponent.K2_SetRelativeLocation` (`self.WallMesh`) (5.0 5.0 400.0) false false))))