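; Destructible prop item that comes in variants such as a crate or chair, chosen by PropsType.
; The construction script sets the static mesh from the PropsSkins array, using PropsType clamped to the array bounds.
; Destroy shakes the given player character's camera, spawns the matching destructible crate or chair Blueprint at the prop's location, then removes the original actor.
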(fn `Destroy`
  (params (PlayerCharacter :type "/Game/Blueprint/Characters/BP_Character_Ogre Object Reference"))
  (`/Game/Blueprint/Characters/BP_Character_Ogre.ShakeCamera` PlayerCharacter)
  (`|SpawnActorFromClass` (select `int` (`self.PropsType`) :`0` "/Game/Blueprint/Props/BP_PropsCaisseDestructible.BP_PropsCaisseDestructible_C" :`1` "/Game/Blueprint/Props/BP_PropsChaise.BP_PropsChaise_C" :!type "Actor Class Reference") (`KismetMathLibrary.MakeTransform` (`self.K2_GetActorLocation`)) "Undefined" "OverrideRootScale" null null)
  (`self.K2_DestroyActor`))

(fn `UserConstructionScript`
  (`StaticMeshComponent.SetStaticMesh` (`self.StaticMesh`) (`|GetArrayItem` (`self.PropsSkins`) (`KismetMathLibrary.Clamp` (`self.PropsType`) 0 (- (`KismetArrayLibrary.Array_Length` (`self.PropsSkins`)) 1)))))