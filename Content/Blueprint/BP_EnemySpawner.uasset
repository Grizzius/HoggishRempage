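; Enemy spawner that spawns grabable enemies from EnemyList at SpawnPoint, one per entry with a delay between each.
; The first overlap on the Awareness sphere, sized by AwarenessRadius in the construction script, caches the player's Ogre, disables further overlaps and starts a wave.
; Each enemy receives the cached player and its Stats entry.
; Tick restarts the wave whenever OnLoop and SpawnReady are true; SpawnReady resets after each completed wave.
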(event `self.ReceiveTick`
  (params (DeltaSeconds :type "Float (single-precision)"))
  (if (and (`self.On Loop`) (`self.SpawnReady`))
    (`self.SpawnEnemies`)))

(event `self.Awareness.OnComponentBeginOverlap`
  (params (OverlappedComponent :type "PrimitiveComponent Object Reference") (OtherActor :type "Actor Object Reference") (OtherComp :type "PrimitiveComponent Object Reference") (OtherBodyIndex :type Integer) (bFromSweep :type Boolean) (SweepResult :type "HitResult Structure (by ref)"))
  (bind _asbp_character_ogre (cast `/Game/Blueprint/Characters/BP_Character_Ogre` (`GameplayStatics.GetPlayerCharacter` 0)))
  (set `self.As BP Character Ogre` _asbp_character_ogre)
  (set `PrimitiveComponent.bGenerateOverlapEvents` false (`self.Awareness`))
  (`self.SpawnEnemies`))

(event `SpawnEnemies`
  (set `self.SpawnReady` false)
  (bind _arrayelement (`/Game/Blueprint/MacroLibrary.ForEachLoopWithDelay` (`self.EnemyList`) (`self.SpawnDelay`))
    (:`LoopBody`
      (`|SpawnActorFromClass` "/Game/Blueprint/Characters/BP_Character_Grabable_Enemy.BP_Character_Grabable_Enemy_C" (`KismetMathLibrary.MakeTransform` (`SceneComponent.K2_GetComponentLocation` (`self.spawn point`))) "Undefined" "OverrideRootScale" null (`self.As BP Character Ogre`) _arrayelement null))
    (:`Completed`
      (set `self.SpawnReady` true))))

(fn `UserConstructionScript`
  (`SphereComponent.SetSphereRadius` (`self.Awareness`) (`KismetMathLibrary.Conv_IntToDouble` (`self.AwarenessRadius`)) true))