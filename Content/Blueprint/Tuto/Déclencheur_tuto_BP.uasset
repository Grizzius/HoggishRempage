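; Tutorial trigger that shows one of three video tutorials the first time its TutoTrigger component is overlapped.
; An AlreadyActivated flag blocks repeat activations, and the overlap does not filter which actor entered.
; TutoIndex selects a matching media player and source to open (Ape, Catfail or Viande), then is passed to a WB_Tuto widget.
; The widget is added to the viewport and the game is paused.
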(event `self.TutoTrigger.OnComponentBeginOverlap`
  (params (OverlappedComponent :type "PrimitiveComponent Object Reference") (OtherActor :type "Actor Object Reference") (OtherComp :type "PrimitiveComponent Object Reference") (OtherBodyIndex :type Integer) (bFromSweep :type Boolean) (SweepResult :type "HitResult Structure (by ref)"))
  (if (not (`self.AlreadyActivated`))
    (set `self.AlreadyActivated` true)
    (`self.OpenTuto` (`self.Tuto Index`))))

(event `OpenTuto`
  (params (TutoIndex :type Integer))
  (bind _tuto_index (`self.Tuto Index`))
  (bind _output_get (set `self.Tuto Index` TutoIndex))
  (`MediaPlayer.OpenSource` (select `int` _tuto_index :`0` "/Game/Blueprint/Tuto/TutoApePlayer.TutoApePlayer" :`1` "/Game/Blueprint/Tuto/TutoCatFailPlayer.TutoCatFailPlayer" :`2` "/Game/Blueprint/Tuto/TutoViandePlayer.TutoViandePlayer" :!type "MediaPlayer Object Reference") (select `int` _tuto_index :`0` "/Game/Blueprint/Tuto/Ape.Ape" :`1` "/Game/Blueprint/Tuto/Catfail.Catfail" :`2` "/Game/Blueprint/Tuto/Viande.Viande" :!type "MediaSource Object Reference"))
  (bind _returnvalue (`|CreateWidget` "/Game/UI/WB_Tuto.WB_Tuto_C" null _output_get))
  (`UserWidget.AddToViewport` _returnvalue 0)
  (`GameplayStatics.SetGamePaused` true))

(fn `UserConstructionScript`)