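; BP_Item_Props is a destructible prop actor with a selectable appearance.
; Its construction script picks the static mesh from the PropsSkins array using PropsType, clamped to a valid index.
; Destroy shakes the passed player character's camera, spawns a scaled-up explosion emitter at the prop's location and removes the actor.
; The event graph holds no active logic, so Destroy relies on an outside caller.
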(fn `Destroy`
  (params (PlayerCharacter :type "/Game/Blueprint/Characters/BP_Character_Ogre Object Reference"))
  (`/Game/Blueprint/Characters/BP_Character_Ogre.ShakeCamera` PlayerCharacter)
  (`GameplayStatics.SpawnEmitterAtLocation` "/Game/StarterContent/Particles/P_Explosion.P_Explosion" (`self.K2_GetActorLocation`) (struct) (2.0 2.0 2.0))
  (`self.K2_DestroyActor`))

(fn `UserConstructionScript`
  (`StaticMeshComponent.SetStaticMesh` (`self.StaticMesh`) (`|GetArrayItem` (`self.PropsSkins`) (`KismetMathLibrary.Clamp` (`self.PropsType`) 0 (- (`KismetArrayLibrary.Array_Length` (`self.PropsSkins`)) 1)))))