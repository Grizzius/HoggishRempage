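; Grabbable "Marmute" character that absorbs enemies hitting it at high speed, storing up to two enemy types in Contenu.
; A qualifying overlap shakes the camera, then either records and kills the enemy or, for non-enemies or when full, destroys the Marmute.
; Destruction enables physics, disables grabbing and explodes after a delay.
; Grabbing makes the mesh ignore GameTraceChannel1, restoring blocking shortly after release.
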(event `self.ToggleGrabbed`
  (params (Grabbed :type Boolean))
  (bind _returnvalue (select `bool` Grabbed :`false` "ECR_Block" :`true` "ECR_Ignore" :!type "ECollisionResponse Enum"))
  (switch `ECollisionResponse` _returnvalue
    (:`ECR_Ignore`
      _)
    (:`ECR_Block`
      (`KismetSystemLibrary.Delay` 0.1)))
  (`PrimitiveComponent.SetCollisionResponseToChannel` (`self.StaticMesh`) "ECC_GameTraceChannel1" _returnvalue))

(event `self.StaticMesh.OnComponentBeginOverlap`
  (params (OverlappedComponent :type "PrimitiveComponent Object Reference") (OtherActor :type "Actor Object Reference") (OtherComp :type "PrimitiveComponent Object Reference") (OtherBodyIndex :type Integer) (bFromSweep :type Boolean) (SweepResult :type "HitResult Structure (by ref)"))
  (if (`self.IsHitAtHighSpeed` OtherActor)
    (`self.ShakeCamera`)
    (if (< (`KismetArrayLibrary.Array_Length` (`self.Contenu`)) 2)
      (bind _asbp_character_grabable_enemy (cast `/Game/Blueprint/Characters/BP_Character_Grabable_Enemy` OtherActor)
        (:`then`
          (`KismetArrayLibrary.Array_Set` (`self.Contenu`) (`self.ContenuSize`) (`.EnemyType_12_BA50D9D84577FADD982FA98101D220D3` (break `/Game/Blueprint/Characters/Struct_EnemyStats` (`/Game/Blueprint/Characters/BP_Character_Grabable_Enemy.Stats` _asbp_character_grabable_enemy))) true)
          (`/Game/Blueprint/Characters/BP_Character_Grabable_Enemy.Die` _asbp_character_grabable_enemy)
          (`/Engine/EditorBlueprintResources/StandardMacros.IncrementInt` (`self.ContenuSize`)))
        (:`CastFailed`
          (`self.DestroyMarmute` :!label _label)))
      (else
        (`KismetSystemLibrary.PrintString` "Marmute is full")
        (goto _label)))))

(event `DestroyMarmute`
  (`PrimitiveComponent.SetSimulatePhysics` (`self.CapsuleComponent`) true)
  (set `self.Grabable` false)
  (`KismetSystemLibrary.Delay` 1.0)
  (`GameplayStatics.SpawnEmitterAtLocation` "/Game/StarterContent/Particles/P_Explosion.P_Explosion" (`self.K2_GetActorLocation`) (struct) (2.0 2.0 2.0))
  (`self.K2_DestroyActor`))

(fn `UserConstructionScript`
  (`parent.UserConstructionScript`))