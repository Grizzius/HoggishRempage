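; Grabbable enemy character (swordsman, crossbowman or spearman) that the player's Ogre can grab, hurt by high-speed impacts.
; Stats drive mesh, armor look, weapon and shield in the construction script, plus HP on BeginPlay.
; Tick stops walking at launched speed, acquires the Ogre by distance and hides distant meshes.
; High-speed DeathHitbox overlaps destroy props and deal damage: armor goes first, then HP, ending in blood and explosion.
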(event `self.ReceiveTick`
  (params (DeltaSeconds :type "Float (single-precision)"))
  (bind _charactermovement (`self.CharacterMovement`))
  (`|ExecutionSequence`
    (:`then_0`
      (if (`self.IsAtLaunchedSpeed`)
        (set `CharacterMovementComponent.MaxWalkSpeed` 0.0 _charactermovement)
        (else
          (set `CharacterMovementComponent.MaxWalkSpeed` 350.0 _charactermovement))))
    (:`then_1`
      (`/Engine/EditorBlueprintResources/StandardMacros.IsValid` (`GameplayStatics.GetPlayerCharacter` 0)
        (:`Is Valid`
          (`/Engine/EditorBlueprintResources/StandardMacros.IsValid` (`self.PlayerCharacter`)
            (:`Is Not Valid`
              (if (< (`self.GetDistanceFromOgre`) (`KismetMathLibrary.Conv_IntToDouble` (`.AwarenessRadius_9_6B2F3383466276204C2BAD998CCE7620` (break `/Game/Blueprint/Characters/Struct_EnemyStats` (`self.Stats`)))))
                (bind _asbp_character_ogre (cast `/Game/Blueprint/Characters/BP_Character_Ogre` (`GameplayStatics.GetPlayerCharacter` 0)))
                (set `self.PlayerCharacter` _asbp_character_ogre)))))))
    (:`then_2`
      (`SceneComponent.SetVisibility` (`self.Mesh`) (< (`self.GetDistanceFromOgre`) 2000.0) true))))

(event `self.DeathHitbox.OnComponentBeginOverlap`
  (params (OverlappedComponent :type "PrimitiveComponent Object Reference") (OtherActor :type "Actor Object Reference") (OtherComp :type "PrimitiveComponent Object Reference") (OtherBodyIndex :type Integer) (bFromSweep :type Boolean) (SweepResult :type "HitResult Structure (by ref)"))
  (bind _charactermovement (`self.CharacterMovement`))
  (if (`self.IsHitAtHighSpeed` OtherActor)
    (bind _asbp_item_props (cast `/Game/Blueprint/BP_Item_Props` OtherActor)
      (:`then`
        (bind _asbp_character_ogre (cast `/Game/Blueprint/Characters/BP_Character_Ogre` (`GameplayStatics.GetPlayerCharacter` 0)))
        (`/Game/Blueprint/BP_Item_Props.Destroy` _asbp_item_props _asbp_character_ogre))
      (:`CastFailed`
        _))
    (`self.ShakeCamera`)
    (`KismetSystemLibrary.Delay` 0.1)
    (`self.Damage`)
    (`/Engine/EditorBlueprintResources/StandardMacros.IsValid` _charactermovement
      (:`Is Valid`
        (set `MovementComponent.Velocity` (0.0 0.0 0.0) _charactermovement)))))

(event `self.ToggleGrabbed`
  (params (Grabbed :type Boolean))
  (`PrimitiveComponent.SetCollisionResponseToChannel` (`self.CapsuleComponent`) "ECC_GameTraceChannel1" (select `bool` Grabbed :`false` "ECR_Block" :`true` "ECR_Ignore" :!type "ECollisionResponse Enum")))

(event `self.ReceiveBeginPlay`
  (set `self.HP` (select `/Game/Blueprint/Characters/Enum_EnemyTypes` (`.EnemyType_12_BA50D9D84577FADD982FA98101D220D3` (break `/Game/Blueprint/Characters/Struct_EnemyStats` (`self.Stats`))) :`NewEnumerator2` 2 :`NewEnumerator0` 1 :`NewEnumerator1` 1))
  (`ActorComponent.K2_DestroyComponent` (`self.Awareness`)))

(event `AttackWithSword`
  (bind _grabbed (`self.IsGrabbed?`))
  (if (not _grabbed)
    (bind _asbp_weapon_sword (cast `/Game/Blueprint/Characters/Weapon/BP_Weapon_Sword` (`ChildActorComponent.ChildActor` (`self.Weapon`))))
    (bind _box (`/Game/Blueprint/Characters/Weapon/BP_Weapon_Sword.Box` _asbp_weapon_sword))
    (`PrimitiveComponent.SetCollisionEnabled` _box "QueryAndPhysics")
    (`KismetSystemLibrary.Delay` 0.2)
    (`PrimitiveComponent.SetCollisionEnabled` _box "NoCollision")
    (set `self.IsAttackingWithSword` false)))

(fn `Damage`
  (bind ((`EnemyType_12_BA50D9D84577FADD982FA98101D220D3` _enemytype) (`AwarenessRadius_9_6B2F3383466276204C2BAD998CCE7620` _awarenessradius)) (break `/Game/Blueprint/Characters/Struct_EnemyStats` (`self.Stats`)))
  (`/Engine/EditorBlueprintResources/StandardMacros.IsValid` self
    (:`Is Valid`
      (`KismetSystemLibrary.PrintString` "Ouch")
      (if (`.Armor_7_5A92E9F34DCF7BF023C3F0930C0F2E02` (break `/Game/Blueprint/Characters/Struct_EnemyStats` (`self.Stats`)))
        (set `self.Stats` (make `/Game/Blueprint/Characters/Struct_EnemyStats` _enemytype false _awarenessradius))
        (set `self.Stunned` false :!label _label)
        (else
          (set `self.HP` (- (`self.HP`) 1))
          (`|ExecutionSequence`
            (:`then_0`
              (goto _label))
            (:`then_1`
              (if (== (`self.HP`) 0)
                (`self.Die`)))))))))

(fn `Die`
  ;[1 1 1] Flaque de sang
  (`|SpawnActorFromClass` "/Game/Blueprint/BP_Bloodsplat.BP_Bloodsplat_C" (`KismetMathLibrary.MakeTransform` (`SceneComponent.K2_GetComponentLocation` (`self.DecalPoint`)) (`KismetMathLibrary.MakeRotator` 0.0 0.0 (`KismetMathLibrary.RandomFloatInRange` -180.0 180.0)) (* (`KismetMathLibrary.MakeVector` 1.0 1.0 1.0) (`KismetMathLibrary.RandomFloatInRange` 0.75 1.75))) "Undefined" "OverrideRootScale" null null)
  (`GameplayStatics.SpawnEmitterAtLocation` "/Game/StarterContent/Particles/P_Explosion.P_Explosion" (`self.K2_GetActorLocation`) (struct) (2.0 2.0 2.0))
  (`self.K2_DestroyActor`))

(fn `GetDistanceFromOgre`
  (returns (ReturnValue :type "Float (double-precision)"))
  (bind _returnvalue (`GameplayStatics.GetPlayerCharacter` 0))
  (`/Engine/EditorBlueprintResources/StandardMacros.IsValid` _returnvalue
    (:`Is Valid`
      (return (`KismetMathLibrary.Vector_Distance` (`self.K2_GetActorLocation`) (`self.K2_GetActorLocation` _returnvalue))))))

(fn `IsAtLaunchedSpeed`
  (returns (ReturnValue :type Boolean))
  (return (> (`KismetMathLibrary.VSize` (`self.GetVelocity`)) 1000.0)))

(fn `IsGrabbed?`
  (returns (Grabbed :type Boolean))
  (bind _asbp_character_ogre (cast `/Game/Blueprint/Characters/BP_Character_Ogre` (`GameplayStatics.GetPlayerCharacter` 0)))
  (return (== (`/Game/Blueprint/Characters/BP_Character_Ogre.GrabbedItem` _asbp_character_ogre) self)))

(fn `UserConstructionScript`
  (locals (NewLocalVar_0 :type "MaterialInterface Object Reference" :default "/Engine/EditorMaterials/WidgetMaterial_Current.WidgetMaterial_Current"))
  (bind ((`EnemyType_12_BA50D9D84577FADD982FA98101D220D3` _enemytype)) (break `/Game/Blueprint/Characters/Struct_EnemyStats` (`self.Stats`)))
  (bind ((`EnemyType_12_BA50D9D84577FADD982FA98101D220D3` _enemytype_2) (`Armor_7_5A92E9F34DCF7BF023C3F0930C0F2E02` _armor)) (break `/Game/Blueprint/Characters/Struct_EnemyStats` (`self.Stats`)))
  (`|ExecutionSequence`
    (:`then_0`
      (if _armor
        (`SkinnedMeshComponent.SetSkinnedAssetAndUpdate` (`self.Mesh`) "/Game/Europe/Knight/Blue/With_Armor/Blue_Knight.Blue_Knight" true)
        (`PrimitiveComponent.SetMaterial` (`self.Mesh`) 0 (select `/Game/Blueprint/Characters/Enum_EnemyTypes` _enemytype_2 :`NewEnumerator2` "/Game/Europe/Knight/Blue/With_Armor/Textur_Bleu_Knight.Textur_Bleu_Knight" :`NewEnumerator0` "/Game/Europe/Knight/Yellow/Armor/Textur_Yellow_Knight.Textur_Yellow_Knight" :`NewEnumerator1` "/Game/Europe/Knight/Green/Armor/Textur_Green_Knight.Textur_Green_Knight" :!type "MaterialInterface Object Reference"))
        (`SkeletalMeshComponent.SetAnimInstanceClass` (`self.Mesh`) null)
        (else
          (`SkinnedMeshComponent.SetSkinnedAssetAndUpdate` (`self.Mesh`) "/Game/Europe/Knight/Blue/Without_armor/Blue_no_Armor.Blue_no_Armor" true)
          (`SkeletalMeshComponent.SetAnimInstanceClass` (`self.Mesh`) null)
          (`PrimitiveComponent.SetMaterial` (`self.Mesh`) 0 (select `/Game/Blueprint/Characters/Enum_EnemyTypes` (`.EnemyType_12_BA50D9D84577FADD982FA98101D220D3` (break `/Game/Blueprint/Characters/Struct_EnemyStats` (`self.Stats`))) :`NewEnumerator2` "/Game/Europe/Knight/Blue/Without_armor/Bue_No_Armor.Bue_No_Armor" :`NewEnumerator0` "/Game/Europe/Knight/Yellow/No_armor/Textur_Yellow_NO_Armor.Textur_Yellow_NO_Armor" :`NewEnumerator1` "/Engine/EditorMaterials/WidgetMaterial_X.WidgetMaterial_X" :!type "MaterialInterface Object Reference")))))
    (:`then_1`
      (`ChildActorComponent.SetChildActorClass` (`self.Weapon`) (select `/Game/Blueprint/Characters/Enum_EnemyTypes` _enemytype :`NewEnumerator2` "/Game/Blueprint/Characters/Weapon/BP_Weapon_Sword.BP_Weapon_Sword_C" :`NewEnumerator0` "/Game/Blueprint/Characters/Weapon/BP_Weapon_CrossBow.BP_Weapon_CrossBow_C" :`NewEnumerator1` "/Game/Blueprint/Characters/Weapon/BP_Weapon_Spear.BP_Weapon_Spear_C" :!type "Actor Class Reference"))
      (`StaticMeshComponent.SetStaticMesh` (`self.WeaponMesh`) (select `/Game/Blueprint/Characters/Enum_EnemyTypes` _enemytype :`NewEnumerator2` "/Game/Europe/Knight/Blue/With_Armor/Weapons/Sword/Sword.Sword" :`NewEnumerator1` "/Game/Blueprint/Characters/Weapon/SM_Weapon_Spear.SM_Weapon_Spear" :!type "StaticMesh Object Reference"))
      (switch `/Game/Blueprint/Characters/Enum_EnemyTypes` _enemytype
        (:`NewEnumerator2`
          _)
        (:`NewEnumerator0`
          _)
        (:`NewEnumerator1`
          (`SceneComponent.K2_SetRelativeRotation` (`self.WeaponMesh`) (struct :`Yaw` -45.0) false false)))
      (`StaticMeshComponent.SetStaticMesh` (`self.ShieldMesh`) (select `/Game/Blueprint/Characters/Enum_EnemyTypes` _enemytype :`NewEnumerator2` "/Game/Europe/Knight/Blue/With_Armor/Weapons/Shield/Shield.Shield" :!type "StaticMesh Object Reference")))
    (:`then_2`
      (`SphereComponent.SetSphereRadius` (`self.Awareness`) (`KismetMathLibrary.Conv_IntToDouble` (`.AwarenessRadius_9_6B2F3383466276204C2BAD998CCE7620` (break `/Game/Blueprint/Characters/Struct_EnemyStats` (`self.Stats`)))) false))))