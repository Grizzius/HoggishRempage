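; Grabbable table that the ogre can carry and that breaks apart on high-speed impacts.
; Construction scatters random physics-simulated tableware over its surface.
; Fast hits destroy props and shake the camera; a held table loses HP and is released at zero, while an unheld one breaks immediately, revealing two physics halves before removal.
; Grabbing toggles a collision channel, delaying the return to Block on release.
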(event `self.ToggleGrabbed`
  (params (Grabbed :type Boolean))
  (bind _returnvalue (select `bool` Grabbed :`false` "ECR_Block" :`true` "ECR_Ignore" :!type "ECollisionResponse Enum"))
  (switch `ECollisionResponse` _returnvalue
    (:`ECR_Ignore`
      _)
    (:`ECR_Block`
      (`KismetSystemLibrary.Delay` 0.1)))
  (`PrimitiveComponent.SetCollisionResponseToChannel` (`self.Box`) "ECC_GameTraceChannel1" _returnvalue))

(event `self.Box.OnComponentBeginOverlap`
  (params (OverlappedComponent :type "PrimitiveComponent Object Reference") (OtherActor :type "Actor Object Reference") (OtherComp :type "PrimitiveComponent Object Reference") (OtherBodyIndex :type Integer) (bFromSweep :type Boolean) (SweepResult :type "HitResult Structure (by ref)"))
  (bind _staticmesh (`self.StaticMesh`))
  (bind _tablepart2 (`self.TablePart2`))
  (if (`self.IsHitAtHighSpeed` OtherActor)
    (`KismetSystemLibrary.PrintString` "Hello")
    (bind _asbp_item_props (cast `/Game/Blueprint/Props/BP_Item_Props` OtherActor)
      (:`then`
        (`/Game/Blueprint/Props/BP_Item_Props.Destroy` _asbp_item_props null))
      (:`CastFailed`
        _))
    (`self.ShakeCamera`)
    (bind _asbp_character_ogre (cast `/Game/Blueprint/Characters/BP_Character_Ogre` (`GameplayStatics.GetPlayerCharacter` 0)))
    (if (== (`/Game/Blueprint/Characters/BP_Character_Ogre.GrabbedItem` _asbp_character_ogre) self)
      (bind _output_get (set `self.HP` (- (`self.HP`) 1)))
      (if (== _output_get 0)
        (`/Game/Blueprint/Characters/BP_Character_Ogre.FreeEbemy` _asbp_character_ogre)
        (`/Engine/EditorBlueprintResources/StandardMacros.IsValid` _staticmesh :!label _label
          (:`Is Valid`
            (`ActorComponent.K2_DestroyComponent` _staticmesh))
          (:`Is Not Valid`
            _))
        (set `self.Grabable` false)
        (`SceneComponent.SetVisibility` _tablepart2 true false)
        (`SceneComponent.SetVisibility` (`self.TablePart1`) true false)
        (`PrimitiveComponent.SetSimulatePhysics` _tablepart2 true)
        (`PrimitiveComponent.SetSimulatePhysics` (`self.TablePart1`) true)
        (`PrimitiveComponent.SetCollisionEnabled` _tablepart2 "QueryAndPhysics")
        (`PrimitiveComponent.SetCollisionEnabled` (`self.TablePart1`) "QueryAndPhysics")
        (`KismetSystemLibrary.Delay` 2.0)
        (`self.K2_DestroyActor`))
      (else
        (goto _label)))))

(fn `UserConstructionScript`
  (for _ (range (+ (`KismetMathLibrary.RandomIntegerInRange` 5 15) 1))
    (bind _returnvalue (`AddComponent|NODE_AddStaticMeshComponent-0` :`RelativeTransform` (`KismetMathLibrary.MakeTransform` (+ (`SceneComponent.RelativeLocation` (`self.Plane`)) (`KismetMathLibrary.MakeVector` (`KismetMathLibrary.RandomFloatInRange` -50.0 50.0) (`KismetMathLibrary.RandomFloatInRange` -130.0 130.0))) (struct) (2.0 2.0 2.0))))
    (`PrimitiveComponent.SetCollisionResponseToChannel` _returnvalue "ECC_GameTraceChannel6" "ECR_Block")
    (`PrimitiveComponent.SetSimulatePhysics` _returnvalue true)
    (`PrimitiveComponent.SetCollisionResponseToChannel` _returnvalue "ECC_GameTraceChannel1" "ECR_Ignore")
    (`StaticMeshComponent.SetStaticMesh` _returnvalue (`|GetArrayItem` (`self.vaisselle`) (`KismetMathLibrary.RandomIntegerInRange` 0 (`KismetArrayLibrary.Array_Length` (`self.vaisselle`)))))))