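; BP_Character_Grabable is a character Blueprint that can be grabbed.
; ToggleGrabbed sets the capsule to ignore a custom collision channel (GameTraceChannel1) while grabbed and to block it otherwise.
; IsHitAtHighSpeed checks whether its own speed plus another actor's exceeds a fixed threshold, ignoring direction.
; ShakeCamera forwards to the player's BP_Character_Ogre to shake the camera.
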(event `ToggleGrabbed`
  (params (Grabbed :type Boolean))
  (`PrimitiveComponent.SetCollisionResponseToChannel` (`self.CapsuleComponent`) "ECC_GameTraceChannel1" (select `bool` Grabbed :`false` "ECR_Block" :`true` "ECR_Ignore" :!type "ECollisionResponse Enum")))

(fn `IsHitAtHighSpeed`
  (params (Other :type "Actor Object Reference"))
  (returns (ReturnValue :type Boolean))
  (`/Engine/EditorBlueprintResources/StandardMacros.IsValid` Other
    (:`Is Valid`
      (return (> (+ (`KismetMathLibrary.VSize` (`self.GetVelocity` Other)) (`KismetMathLibrary.VSize` (`self.GetVelocity`))) 1500.0)))))

(fn `ShakeCamera`
  (bind _asbp_character_ogre (cast `/Game/Blueprint/Characters/BP_Character_Ogre` (`GameplayStatics.GetPlayerCharacter` 0)))
  (`/Game/Blueprint/Characters/BP_Character_Ogre.ShakeCamera` _asbp_character_ogre))

(fn `UserConstructionScript`)