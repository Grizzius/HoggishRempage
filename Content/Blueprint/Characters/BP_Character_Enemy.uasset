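; BP_Character_Enemy is an enemy character whose type (Arbaletrier, Lancier, Epeiste) sets its HP and weapon child actor, and, with armor, its material.
; It can be grabbed and launched: at launch speed walking stops, and death-hitbox overlaps damage it and any enemy hit, shaking the Ogre player's camera.
; Armor absorbs one hit before HP drops, and death spawns a blood splat.
; Awareness overlaps track the Ogre, and sword attacks briefly enable the blade's collision.
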(event `ToggleGrabbed`
  (params (Grabbed :type Boolean))
  (`PrimitiveComponent.SetCollisionEnabled` (`self.CapsuleComponent`) (select `bool` Grabbed :`false` "QueryAndPhysics" :`true` "NoCollision" :!type "ECollisionEnabled Enum")))

(event `self.DeathHitbox.OnComponentBeginOverlap`
  (params (OverlappedComponent :type "PrimitiveComponent Object Reference") (OtherActor :type "Actor Object Reference") (OtherComp :type "PrimitiveComponent Object Reference") (OtherBodyIndex :type Integer) (bFromSweep :type Boolean) (SweepResult :type "HitResult Structure (by ref)"))
  (bind _charactermovement (`self.CharacterMovement`))
  (if (`self.IsAtLaunchedSpeed`)
    (bind _asbp_character_enemy (cast `/Game/Blueprint/Characters/BP_Character_Enemy` OtherActor)
      (:`then`
        (`self.Damage` _asbp_character_enemy))
      (:`CastFailed`
        _))
    (`self.ShakeCamera`)
    (`KismetSystemLibrary.Delay` 0.1)
    (`self.Damage`)
    (`/Engine/EditorBlueprintResources/StandardMacros.IsValid` _charactermovement
      (:`Is Valid`
        (set `MovementComponent.Velocity` (0.0 0.0 0.0) _charactermovement)))))

(event `self.Awareness.OnComponentBeginOverlap`
  (params (OverlappedComponent :type "PrimitiveComponent Object Reference") (OtherActor :type "Actor Object Reference") (OtherComp :type "PrimitiveComponent Object Reference") (OtherBodyIndex :type Integer) (bFromSweep :type Boolean) (SweepResult :type "HitResult Structure (by ref)"))
  (bind _asbp_character_ogre (cast `/Game/Blueprint/Characters/BP_Character_Ogre` OtherActor))
  (set `self.PlayerCharacter` _asbp_character_ogre))

(event `self.Awareness.OnComponentEndOverlap`
  (params (OverlappedComponent :type "PrimitiveComponent Object Reference") (OtherActor :type "Actor Object Reference") (OtherComp :type "PrimitiveComponent Object Reference") (OtherBodyIndex :type Integer))
  (set `self.PlayerCharacter` null))

(event `self.ReceiveBeginPlay`
  (set `self.HP` (select `/Game/Blueprint/Characters/Enum_EnemyTypes` (`self.EnemyType`) :`NewEnumerator0` 1 :`NewEnumerator1` 1 :`NewEnumerator2` 2)))

(event `self.ReceiveTick`
  (params (DeltaSeconds :type "Float (single-precision)"))
  (bind _charactermovement (`self.CharacterMovement`))
  (if (`self.IsAtLaunchedSpeed`)
    (set `CharacterMovementComponent.MaxWalkSpeed` 0.0 _charactermovement)
    (else
      (set `CharacterMovementComponent.MaxWalkSpeed` 350.0 _charactermovement))))

(event `AttackWithSword`
  (bind _asbp_weapon_sword (cast `/Game/Blueprint/Characters/Weapon/BP_Weapon_Sword` (`ChildActorComponent.ChildActor` (`self.Weapon`))))
  (bind _box (`/Game/Blueprint/Characters/Weapon/BP_Weapon_Sword.Box` _asbp_weapon_sword))
  (`PrimitiveComponent.SetCollisionEnabled` _box "QueryAndPhysics")
  (`KismetSystemLibrary.Delay` 0.2)
  (`PrimitiveComponent.SetCollisionEnabled` _box "NoCollision"))

(fn `Damage`
  (`/Engine/EditorBlueprintResources/StandardMacros.IsValid` self
    (:`Is Valid`
      (`KismetSystemLibrary.PrintString` "Ouch")
      (if (`self.Armor`)
        (set `self.Armor` false)
        (else
          (set `self.HP` (- (`self.HP`) 1))
          (if (== (`self.HP`) 0)
            ;[1 1 1] Flaque de sang
            (`|SpawnActorFromClass` "/Game/Blueprint/BP_Bloodsplat.BP_Bloodsplat_C" (`KismetMathLibrary.MakeTransform` (`SceneComponent.K2_GetComponentLocation` (`self.DecalPoint`)) (`KismetMathLibrary.MakeRotator` 0.0 0.0 (`KismetMathLibrary.RandomFloatInRange` -180.0 180.0)) (* (`KismetMathLibrary.MakeVector` 1.0 1.0 1.0) (`KismetMathLibrary.RandomFloatInRange` 0.75 1.75))) "Undefined" "OverrideRootScale" null null)
            (`self.K2_DestroyActor`)))))))

(fn `IsAtLaunchedSpeed`
  (returns (ReturnValue :type Boolean))
  (return (> (`KismetMathLibrary.VSize` (`self.GetVelocity`)) 1000.0)))

(fn `ShakeCamera`
  (bind _asbp_character_ogre (cast `/Game/Blueprint/Characters/BP_Character_Ogre` (`GameplayStatics.GetPlayerCharacter` 0)))
  (`/Game/Blueprint/Characters/BP_Character_Ogre.ShakeCamera` _asbp_character_ogre))

(fn `UserConstructionScript`
  (locals (NewLocalVar_0 :type "MaterialInterface Object Reference" :default "/Engine/EditorMaterials/WidgetMaterial_Current.WidgetMaterial_Current"))
  (`|ExecutionSequence`
    (:`then_0`
      (if (`self.Armor`)
        (`PrimitiveComponent.SetMaterial` (`self.Mesh`) 0 (select `/Game/Blueprint/Characters/Enum_EnemyTypes` (`self.EnemyType`) :`NewEnumerator0` "/Engine/EditorMaterials/Cloth/CameraLitDoubleSided.CameraLitDoubleSided" :`NewEnumerator1` "/Engine/MapTemplates/Materials/BasicAsset01.BasicAsset01" :`NewEnumerator2` "/Engine/VREditor/Teleport/TeleportDirectionMaterial.TeleportDirectionMaterial" :!type "MaterialInterface Object Reference"))
        (else
          (`PrimitiveComponent.SetMaterial` (`self.Mesh`) 0 (select `/Game/Blueprint/Characters/Enum_EnemyTypes` (`self.EnemyType`) :`NewEnumerator0` "/Engine/EditorMaterials/WidgetMaterial_Current.WidgetMaterial_Current" :`NewEnumerator1` "/Engine/EditorMaterials/WidgetMaterial_X.WidgetMaterial_X" :`NewEnumerator2` "/Engine/EditorMaterials/WidgetMaterial_Z.WidgetMaterial_Z" :!type "MaterialInterface Object Reference")))))
    (:`then_1`
      (`ChildActorComponent.SetChildActorClass` (`self.Weapon`) (select `/Game/Blueprint/Characters/Enum_EnemyTypes` (`self.EnemyType`) :`NewEnumerator1` "/Game/Blueprint/Characters/Weapon/BP_Weapon_Spear.BP_Weapon_Spear_C" :`NewEnumerator2` "/Game/Blueprint/Characters/Weapon/BP_Weapon_Sword.BP_Weapon_Sword_C" :!type "Actor Class Reference")))))